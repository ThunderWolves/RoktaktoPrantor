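; Enemy character Blueprint that chases and melee-attacks the player, with a widget health HUD bound to itself.
; Overlap with the player toggles range and starts or stops an AI MoveTo chase loop; arrival plays an attack montage and, after a delay, damages the player if still close.
; Damage taken is bone-based: headshots kill instantly, other hits subtract health, play a stagger, then resume the chase or trigger death.
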(event Custom|Chase%20the%20player
  (bind _bp_base (Variables|Default|Getbp_base))
  (bind _returnvalue (Transformation|GetDistanceTo _bp_base))
  (if (!= (Variables|Default|GetCurrentheath) 0.0)
    (Development|PrintString "accHello")
    (AI|AIMoveTo self "0, 0, 0" (Game|GetPlayerCharacter 0) 1e+02 false
      (:OnSuccess
        (if (Variables|Default|GetCan%20attack)
          (Variables|Default|SetCan%20attack false)
          (Animation|Montage|PlayMontage (Variables|Character|GetMesh) "/Game/Enemy_aladin/Aladin_attack_mont.Aladin_attack_mont"
            (:then
              (Utilities|FlowControl|Delay 0.85)
              (Development|PrintString (Utilities|String|ToString(Float) _returnvalue))
              (if (< _returnvalue 156.0)
                (bind _asbp_base (Utilities|Casting|CastToBP_base _bp_base))
                (Variables|/Game/Blueprint/BP_base.BP_base_C|Setcurrenthealth _asbp_base (- (Variables|/Game/Blueprint/BP_base.BP_base_C|Getcurrenthealth _asbp_base) 0.2))))
            (:OnCompleted
              (Variables|Default|SetCan%20attack true)
              (if (Variables|Default|GetPlayer%20in%20range)
                (CallFunction|ChasethePlayer))))
          (else
            (CallFunction|ChasethePlayer))))
      (:OnFail
        (Development|PrintString "2")))))

(event Custom|CustomEvent
  (params (BoneName :type Name)))

(event EventItakedamage
  (params (BoneName :type Name :default "None"))
  (if (!= (Variables|Default|GetCurrentheath) 0.0)
    (if (Utilities|Name|Equal(Name) BoneName "Head")
      (Variables|Default|SetCurrentheath 0.0)
      (Components|Animation|PlayAnimation (Variables|Character|GetMesh) "/Game/Enemy_aladin/Animation/Death_From_Back_Headshot.Death_From_Back_Headshot" false)
      (Class|Pawn|DetachfromControllerPendingDestroy :!label _label)
      (else
        (bind _output_get (Variables|Default|SetCurrentheath (- (Variables|Default|GetCurrentheath) 0.3)))
        (if (<= _output_get 0.0)
          (Variables|Default|SetCurrentheath 0.0)
          (Components|Animation|PlayAnimation (Variables|Character|GetMesh) "/Game/Enemy_aladin/Animation/Dying.Dying" false)
          (goto _label)
          (else
            (Components|Animation|PlayAnimation (Variables|Character|GetMesh) "/Game/Enemy_aladin/Animation/Head_Hit.Head_Hit" false)
            (Components|Movement|StopMovementImmediately (Variables|Character|GetCharacterMovement))
            (Utilities|FlowControl|Delay 1.23)
            (if (!= (Variables|Default|GetCurrentheath) 0.0)
              (Components|Animation|SetAnimationMode (Variables|Character|GetMesh) "AnimationBlueprint")
              (Development|PrintString "Hello")
              (CallFunction|ChasethePlayer))))))))

(event Collision|EventActorBeginOverlap
  (params (OtherActor :type Actor%20Object%20Reference))
  (if (!= (Variables|Default|GetCurrentheath) 0.0)
    (Utilities|Casting|CastToBP_base OtherActor)
    (Variables|Default|SetPlayer%20in%20range true)
    (CallFunction|ChasethePlayer)))

(event EventBeginPlay
  (bind _asai_hud (Utilities|Casting|CastToAI_HUD (UserInterface|GetUserWidgetObject (Variables|Default|GetWidget))))
  (Variables|/Game/Blueprint/AI_HUD.AI_HUD_C|Setowner _asai_hud self)
  (Variables|Default|Setbp_base (Game|GetPlayerCharacter 0)))

(event Collision|EventActorEndOverlap
  (params (OtherActor :type Actor%20Object%20Reference))
  (if (!= (Variables|Default|GetCurrentheath) 0.0)
    (Utilities|Casting|CastToBP_base OtherActor)
    (Variables|Default|SetPlayer%20in%20range false)
    (Components|Movement|StopMovementImmediately (Variables|Character|GetCharacterMovement))))

(fn ConstructionScript)